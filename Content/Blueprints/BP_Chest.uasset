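; BP_Chest is an interactable chest that shows a PressE prompt while the third-person character overlaps its box.
; Interface-style open and close events share logic with OpenLit and CloseLit.
; Opening plays a sound and a timeline that slides the lid along world X from its BeginPlay location, with an automatic close delayed from the timeline's update.
; Closing waits briefly, plays a sound and snaps the lid back.
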(event OnComponentBeginOverlap(Box)
  (params (OverlappedComponent :type Primitive%20Component%20Object%20Reference) (OtherActor :type Actor%20Object%20Reference) (OtherComp :type Primitive%20Component%20Object%20Reference) (OtherBodyIndex :type Integer) (bFromSweep :type Boolean) (SweepResult :type Hit%20Result%20Structure%20%28by%20ref%29))
  (Utilities|Casting|CastToBP_ThirdPersonCharacter OtherActor)
  (Rendering|SetVisibility (Variables|Default|GetPress%20E) true false))

(event OnComponentEndOverlap(Box)
  (params (OverlappedComponent :type Primitive%20Component%20Object%20Reference) (OtherActor :type Actor%20Object%20Reference) (OtherComp :type Primitive%20Component%20Object%20Reference) (OtherBodyIndex :type Integer))
  (Utilities|Casting|CastToBP_ThirdPersonCharacter OtherActor)
  (Rendering|SetVisibility (Variables|Default|GetPress%20E) false false))

(event Custom|CloseLit
  (Utilities|FlowControl|Delay 0.5)
  (Audio|PlaySound2D "/Game/Sounds/SFX/SC_ChestClose.SC_ChestClose" 1.0 1.0 0.0 0 0)
  (Transformation|SetWorldLocation (Variables|Default|GetLit) (Variables|Default|GetLit%20Location) true false))

(event Custom|Open%20Lit
  (bind _lit_location (Variables|Default|GetLit%20Location))
  (Utilities|FlowControl|Sequence
    (:then_0
      (Audio|PlaySound2D "/Game/Sounds/SFX/SC_ChestOpen.SC_ChestOpen" 1.0 1.0 0.0 0 0))
    (:then_1
      (bind _litopen (Timeline|OpenChest PlayFromStart)
        (:Update
          (Transformation|SetWorldLocation (Variables|Default|GetLit) (Math|Vector|Lerp(Vector) _lit_location (+ _lit_location "-50.000000,0.000000,0.000000") _litopen) true false)
          (Utilities|FlowControl|Delay 5.0)
          (CallFunction|CloseLit))))))

(event EventBeginPlay
  (Variables|Default|SetLit%20Location (Transformation|GetWorldLocation (Variables|Default|GetLit))))

(event Collision|EventActorBeginOverlap
  (params (OtherActor :type Actor%20Object%20Reference)))

(event EventTick
  (params (DeltaSeconds :type Float%20%28single-precision%29)))

(event EventOpenChestBPI
  (bind _lit_location (Variables|Default|GetLit%20Location))
  (Utilities|FlowControl|Sequence
    (:then_0
      (Audio|PlaySound2D "/Game/Sounds/SFX/SC_ChestOpen.SC_ChestOpen" 1.0 1.0 0.0 0 0))
    (:then_1
      (bind _litopen (Timeline|OpenChest PlayFromStart)
        (:Update
          (Transformation|SetWorldLocation (Variables|Default|GetLit) (Math|Vector|Lerp(Vector) _lit_location (+ _lit_location "-50.000000,0.000000,0.000000") _litopen) true false)
          (Utilities|FlowControl|Delay 5.0)
          (CallFunction|CloseLit))))))

(event EventCloseChestBPI
  (Utilities|FlowControl|Delay 0.5)
  (Audio|PlaySound2D "/Game/Sounds/SFX/SC_ChestClose.SC_ChestClose" 1.0 1.0 0.0 0 0)
  (Transformation|SetWorldLocation (Variables|Default|GetLit) (Variables|Default|GetLit%20Location) true false))

(fn ConstructionScript
  (bind _outactors (Actor|GetAllActorsOfClass "/Game/ThirdPerson/Blueprints/BP_ThirdPersonCharacter.BP_ThirdPersonCharacter_C"))
  (Variables|Default|SetPlayer (Utilities|Array|Get(acopy) _outactors)))