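; NPC that patrols, chases the player, supports conversation hooks and can be stealth-killed and carried.
; AIMoveTo loops between random TargetPoints with alternating montages; PawnSensing sets Player and starts the chase.
; StealthBackKill plays the victim montage and calls Ragdoll, which disables collision without simulating physics and sets IsDead, enabling the pickup prompt and Carry.
; Interaction state toggles the name label, and Tick drains Tired after it reaches MaxTired.
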(event OnSeePawn(PawnSensing)
  (params (Pawn :type Pawn%20Object%20Reference))
  ;[1 1 1] Chase Player
  (Collision|LineTraceByChannel (Transformation|GetWorldLocation (Variables|Character|GetMesh)) (Transformation|GetActorLocation Pawn) "TraceTypeQuery2" false 0 "ForDuration")
  (Variables|Default|Setplayer? true)
  (AI|AIMoveTo self "0, 0, 0" (Game|GetPlayerCharacter 0) 5.0 false))

(event OnComponentBeginOverlap(NPCRaduis)
  (params (OverlappedComponent :type Primitive%20Component%20Object%20Reference) (OtherActor :type Actor%20Object%20Reference) (OtherComp :type Primitive%20Component%20Object%20Reference) (OtherBodyIndex :type Integer) (bFromSweep :type Boolean) (SweepResult :type Hit%20Result%20Structure%20%28by%20ref%29))
  ;[1 1 1] PICK UP MUERTO
  (Utilities|Casting|CastToBP_ThirdPersonCharacter OtherActor)
  (if (Variables|Default|GetisDead?)
    (Rendering|SetVisibility (Variables|Default|GetPickUp_F) true false)))

(event OnComponentEndOverlap(NPCRaduis)
  (params (OverlappedComponent :type Primitive%20Component%20Object%20Reference) (OtherActor :type Actor%20Object%20Reference) (OtherComp :type Primitive%20Component%20Object%20Reference) (OtherBodyIndex :type Integer))
  ;[1 1 1] PICK UP MUERTO
  (Utilities|Casting|CastToBP_ThirdPersonCharacter OtherActor)
  (if (Variables|Default|GetisDead?)
    (Rendering|SetVisibility (Variables|Default|GetPickUp_F) false false)))

(event Custom|Ragdoll
  ;[1 1 1] Dead
  (Audio|Components|Audio|SetVolumeMultiplier (Variables|Default|GetSC_NPC) 0.0 :!class /Script/Engine.AudioComponent)
  (Audio|PlaySound2D "/Game/Sounds/NPCs/SC_Die.SC_Die" 1.0 1.0 0.0 0 0)
  (Utilities|FlowControl|Delay 2.5)
  (Variables|Default|SetisDead? true)
  (Collision|SetCollisionResponsetoChannel (Variables|Collision|GetCapsuleComponent) "ECC_Pawn" "ECR_Overlap")
  (Collision|SetCollisionEnabled (Variables|Character|GetMesh) "NoCollision"))

(event Custom|Patrol
  (bind _mesh (Variables|Character|GetMesh))
  ;[1 1 1] PAtrol
  (if (not (Variables|Default|Getplayer?))
    (AI|AIMoveTo self "0, 0, 0" (.OutItem (Utilities|Array|Random (Variables|Default|GetTargetPoint))) 5.0 false :!label _label
      (:OnSuccess
        (Utilities|FlowControl|FlipFlop
          (:A
            (Animation|Montage|PlayMontage _mesh "/Game/Animations/Montages/Convo_01_Low_Key_Loop_Montage.Convo_01_Low_Key_Loop_Montage"
              (:OnCompleted
                _)))
          (:B
            (Animation|Montage|PlayMontage _mesh "/Game/Animations/Montages/Convo_11_Listening_Loop_Montage.Convo_11_Listening_Loop_Montage"
              (:OnCompleted
                _))))
        (Utilities|FlowControl|Delay 3.0)
        (goto _label)))))

(event Custom|IncreaseTired
  (Variables|Default|SetTired (+ (Variables|Default|GetTired) (Variables|Character|GetTiredAmount))))

(event EventBeginPlay
  ;[1 1 1] Begin Patrol
  (CallFunction|Patrol))

(event EventTick
  (params (DeltaSeconds :type Float%20%28single-precision%29))
  (if (>= (Variables|Default|GetTired) (Variables|Default|GetMaxTired))
    (Utilities|FlowControl|Delay 1e+01)
    (Variables|Default|SetTired (- (Variables|Default|GetTired) 0.1) :!label _label)
    (if (not (<= (Variables|Default|GetTired) 0.0))
      (Utilities|FlowControl|Delay 1.0)
      (goto _label))))

(event EventSetInteractableState
  (params (bCanShowInteract? :type Boolean))
  ;[1 1 1] Conversacion
  (if bCanShowInteract?
    (Rendering|SetVisibility (Variables|Default|GetNPC_Name) true false)
    (else
      (Rendering|SetVisibility (Variables|Default|GetNPC_Name) false false))))

(event EventConversationClosed
  ;[1 1 1] Conversacion
  (Class|BPIInteractable|ConversationClosed(Message) (Variables|Default|GetInteractIntigator)))

(fn ConstructionScript
  (Rendering|Components|TextRender|SetText (Variables|Default|GetNPC_Name) (Variables|Default|GetNPCName)))

(fn Carry
  (if (Variables|Default|GetisDead?)
    (Rendering|SetVisibility (Variables|Character|GetMesh) false true)
    (Collision|SetCollisionEnabled (Variables|Default|GetPlayerInteractionsRaduis) "NoCollision")
    (Collision|SetCollisionEnabled (Variables|Default|GetNPCRaduis) "NoCollision")
    (return (Transformation|GetWorldLocation (Variables|Default|GetPlayerKill)) (Transformation|GetActorRotation))))

(fn StealthBackKill
  (if (not (Variables|Default|GetisDead?))
    (Animation|PlayAnimMontage "/Game/Animations/Montages/Paired_Knife_Stealth_KidneyAndNeck_Vic_Montage.Paired_Knife_Stealth_KidneyAndNeck_Vic_Montage" 1.0 "None")
    (CallFunction|Ragdoll)
    (return (Transformation|GetWorldLocation (Variables|Default|GetPlayerKill)) (Transformation|GetActorRotation))))