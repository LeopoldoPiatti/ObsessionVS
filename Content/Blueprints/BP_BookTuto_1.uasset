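; BP_BookTuto_1 is a Blueprint that shows a book tutorial widget, WB_BookTuto_11, on screen.
; On BeginPlay it creates the widget, stores it, adds it to the viewport and switches input to game and UI with the mouse cursor visible.
; Its Remove event takes the widget off screen, hides the cursor and restores game-only input.
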(event Custom|Remove
  (bind _returnvalue (Game|GetPlayerController 0))
  (Widget|RemovefromParent (Variables|Default|GetWB_Book_1))
  (Variables|/Script/Engine.PlayerController|SetbShowMouseCursor _returnvalue false)
  (Input|SetInputModeGameOnly _returnvalue false))

(event EventBeginPlay
  (bind _returnvalue (Game|GetPlayerController 0))
  (bind _returnvalue_2 (UserInterface|CreateWidget "/Game/Blueprints/UI/WB_BookTuto_1-1.WB_BookTuto_1-1_C" _returnvalue))
  (bind _output_get (Variables|Default|SetWB_Book_1 _returnvalue_2))
  (UserInterface|Viewport|AddtoViewport _returnvalue_2 0)
  (Input|SetInputModeGameandUI _returnvalue 0 "DoNotLock" true false)
  (Variables|/Script/Engine.PlayerController|SetbShowMouseCursor _returnvalue true))

(fn ConstructionScript)