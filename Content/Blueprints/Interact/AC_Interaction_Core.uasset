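; Base interaction component that detects the actor under the screen centre for its owner to interact with.
; TraceForInteract line-traces from the deprojected viewport centre, adding the camera-to-owner distance to InteractDistance so camera offset does not shorten reach.
; Target changes track current and previous actors, reset hold duration and call UpdateInteractState, an empty hook here.
; A recheck flag re-fires that update on an unchanged target.
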(fn GetTraceLocations
  (bind _returnvalue (Viewport|GetViewportSize))
  (bind _returnvalue_2 (Game|GetPlayerController 0))
  (bind _returnvalue_3 (/ _returnvalue "(X=2.000000,Y=2.000000)"))
  (bind (_worldposition _worlddirection) (Class|GameplayStatics|DeprojectScreentoWorld _returnvalue_2 _returnvalue_3))
  (return _worldposition (+ _worldposition (* (+ (Math|Vector|Distance(Vector) _worldposition (Transformation|GetActorLocation (Components|GetOwner))) (Variables|Default|GetInteractDistance)) _worlddirection))))

(fn TraceforInteract
  (bind (_start _end) (CallFunction|GetTraceLocations))
  (bind (_outhit _returnvalue) (Collision|LineTraceByChannel _start _end "TraceTypeQuery3" false 0 "None"))
  (if _returnvalue
    (if (!= (.HitActor (Collision|BreakHitResult _outhit)) (Variables|Default|GetCurrentHitActor))
      (Variables|Default|SetPrevHitActor (Variables|Default|GetCurrentHitActor))
      (Variables|Default|SetCurrentHitActor (.HitActor (Collision|BreakHitResult _outhit)))
      (Variables|Default|SetbCanSetPrevious? true)
      (Variables|Default|SetCurrentHoldDuration 0.0)
      (CallFunction|UpdateInteractState true :!label _label)
      (elif (CallFunction|GetRecheckHit)
        (CallFunction|DisableHitRecheck)
        (goto _label)))
    (elif (Variables|Default|GetbCanSetPrevious?)
      (CallFunction|DisableHitRecheck)
      (Utilities|IsValid (Variables|Default|GetCurrentHitActor)
        (:Is%20Valid
          (Variables|Default|SetPrevHitActor (Variables|Default|GetCurrentHitActor)))
        (:Is%20Not%20Valid
          (Variables|Default|SetPrevHitActor 0)))
      (Variables|Default|SetCurrentHitActor 0)
      (Variables|Default|SetbCanSetPrevious? false)
      (Variables|Default|SetCurrentHoldDuration 0.0)
      (CallFunction|UpdateInteractState false))))

(fn UpdateInteractState
  (params (bHit? :type Boolean)))