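; Dialogue component for the NPC Chilampi, scripting a short branching conversation about Sherlock Holmes and a book.
; Overrides the parent's Dialogue, switching on DialogueTreeIndex and nesting AddDialogue blocks that branch on the chosen option.
; Endings advance the tree index, remove or clear dialogue progress, then close the conversation; answering "No" also triggers an aggression dice roll.
; BeginPlay caches the first BP_NPC_V2 found as NPCChilampi; the "Back" option has no handler here.
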(event EventBeginPlay
  (|CallParentFunction)
  (bind _outactors (Actor|GetAllActorsOfClass "/Game/Blueprints/NPCs/BP_NPC_V2.BP_NPC_V2_C"))
  (Variables|Default|SetNPC_Chilampi (Utilities|Array|Get(acopy) _outactors)))

(event EventTick
  (params (DeltaSeconds :type Float%20%28single-precision%29))
  (|CallParentFunction DeltaSeconds) ; This node is disabled and will not be called.\nDrag off pins to build functionality.
)

(fn Dialogue
  (|CallParentFunction)
  (switch int (Variables|Default|GetDialogueTreeIndex)
    (:0
      ;[1 1 1] Bloque de conversacion (0)
      (bind (_state _optionsindex) (CallFunction|AddDialogue "Chilampi" "Hello, do you like Sherlock Holmes?" (Utilities|Array|MakeArray "Hapiness: Yes" "Affection: No" "Back")))
      (switch Utilities|FlowControl|Switch|SwitchonEnum_DialogueState _state
        (:NewEnumerator0
          (switch int _optionsindex
            (:0
              ;[1 1 1] Bloque de conversacion (1)
              (bind (_state_2 _optionsindex_2) (CallFunction|AddDialogue "Chilampi" "Great, I have a book" (Utilities|Array|MakeArray "Give book" "Affection: Not give book")))
              (switch Utilities|FlowControl|Switch|SwitchonEnum_DialogueState _state_2
                (:NewEnumerator0
                  (switch int _optionsindex_2
                    (:0
                      ;[1 1 1] Bloque de conversacion (2)
                      (bind _state_3 (CallFunction|AddDialogue "Chilampi" "Great, I have a book" (Utilities|Array|MakeArray "Cont_1")))
                      (switch Utilities|FlowControl|Switch|SwitchonEnum_DialogueState _state_3
                        (:NewEnumerator0
                          (CallFunction|SetDialogueTreeIndex 1)
                          (CallFunction|CloseConversation))))
                    (:1
                      ;[1 1 1] Bloque de conversacion (2)
                      (bind _state_4 (CallFunction|AddDialogue "Chilampi" "Great, I have a book" (Utilities|Array|MakeArray "Con_2")))
                      (switch Utilities|FlowControl|Switch|SwitchonEnum_DialogueState _state_4
                        (:NewEnumerator0
                          (CallFunction|RemoveDialogueProgress 2)
                          (CallFunction|CloseConversation))))))))
            (:1
              (CallFunction|DiceRollAgresion 1)
              ;[1 1 1] Bloque de conversacion (1)
              (bind _state_5 (CallFunction|AddDialogue "Chilampi" "Too bad, I have a book" (Utilities|Array|MakeArray "I dont wanted")))
              (switch Utilities|FlowControl|Switch|SwitchonEnum_DialogueState _state_5
                (:NewEnumerator0
                  (CallFunction|ClearDialogueProgress)
                  (CallFunction|CloseConversation))))))))))