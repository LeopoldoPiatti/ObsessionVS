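; Dialogue component for the NPC Roman, scripting a branching book-recommendation conversation about Sherlock Holmes on top of a parent dialogue class.
; Dialogue nests AddDialogue blocks four levels deep, where Aggressive and Seduction choices trigger dice rolls numbered by depth.
; Back steps progress back one, while Bye and final choices clear it and close the conversation.
; Several branches repeat lines or hold placeholder text, and BeginPlay caches the first BP_NPC_V2 as NPCChilampi.
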(event EventBeginPlay
  (|CallParentFunction)
  (bind _outactors (Actor|GetAllActorsOfClass "/Game/Blueprints/NPCs/BP_NPC_V2.BP_NPC_V2_C"))
  (Variables|Default|SetNPC_Chilampi (Utilities|Array|Get(acopy) _outactors)))

(event EventTick
  (params (DeltaSeconds :type Float%20%28single-precision%29))
  (|CallParentFunction DeltaSeconds) ; This node is disabled and will not be called.\nDrag off pins to build functionality.
)

(fn Dialogue
  (|CallParentFunction)
  (switch int (Variables|Default|GetDialogueTreeIndex)
    (:0
      ;[1 1 1] Bloque de conversacion (0)
      (bind (_state _optionsindex) (CallFunction|AddDialogue (Variables|Default|GetNPC%20Name) "Hi! Recommendations for an interesting read?" (Utilities|Array|MakeArray "Aggressive: \"A Study in Scarlet\" by Conan Doyle." "Seduction: Prefer something more contemporary? We have some mystery and suspense novels that might grab your attention." "Bye!")))
      (switch Utilities|FlowControl|Switch|SwitchonEnum_DialogueState _state
        (:NewEnumerator0
          (switch int _optionsindex
            (:0
              (CallFunction|DiceRollAgresion 1)
              ;[1 1 1] Bloque de conversacion (1)
              (bind (_state_2 _optionsindex_2) (CallFunction|AddDialogue (Variables|Default|GetNPC%20Name) "Where should I start with Sherlock?" (Utilities|Array|MakeArray "Aggressive: Begin with \"A Study in Scarlet.\"" "Seduction: Try \"A Scandal in Bohemia.\"" "Back")))
              (switch Utilities|FlowControl|Switch|SwitchonEnum_DialogueState _state_2
                (:NewEnumerator0
                  (switch int _optionsindex_2
                    (:0
                      (CallFunction|DiceRollAgresion 2)
                      ;[1 1 1] Bloque de conversacion (2)
                      (bind (_state_3 _optionsindex_3) (CallFunction|AddDialogue (Variables|Default|GetNPC%20Name) "What makes Sherlock special?" (Utilities|Array|MakeArray "Aggressive: Holmes's deductive brilliance." "Seduction: Solving impossible cases." "Back")))
                      (switch Utilities|FlowControl|Switch|SwitchonEnum_DialogueState _state_3
                        (:NewEnumerator0
                          (switch int _optionsindex_3
                            (:0
                              (CallFunction|DiceRollAgresion 3)
                              ;[1 1 1] Bloque de conversacion (3)
                              (bind (_state_4 _optionsindex_4) (CallFunction|AddDialogue (Variables|Default|GetNPC%20Name) "Anything else I should know?" (Utilities|Array|MakeArray " Aggressive: Detailed Victorian narrative." " Seduction: Enjoy Holmes's wit." "Bye!")))
                              (switch Utilities|FlowControl|Switch|SwitchonEnum_DialogueState _state_4
                                (:NewEnumerator0
                                  (switch int _optionsindex_4
                                    (:0
                                      (CallFunction|DiceRollAgresion 4)
                                      (CallFunction|ClearDialogueProgress)
                                      (CallFunction|CloseConversation))
                                    (:1
                                      (CallFunction|DiceRollSeduction 4)
                                      (CallFunction|ClearDialogueProgress)
                                      (CallFunction|CloseConversation))
                                    (:2
                                      (CallFunction|ClearDialogueProgress)
                                      (CallFunction|CloseConversation))))))
                            (:1
                              (CallFunction|DiceRollSeduction 3)
                              ;[1 1 1] Bloque de conversacion (3)
                              (bind (_state_5 _optionsindex_5) (CallFunction|AddDialogue (Variables|Default|GetNPC%20Name) "What makes Sherlock special?" (Utilities|Array|MakeArray "Aggressive: Holmes's deductive brilliance." "Seduction: Solving impossible cases." "Bye!")))
                              (switch Utilities|FlowControl|Switch|SwitchonEnum_DialogueState _state_5
                                (:NewEnumerator0
                                  (switch int _optionsindex_5
                                    (:0
                                      (CallFunction|DiceRollAgresion 4)
                                      (CallFunction|ClearDialogueProgress)
                                      (CallFunction|CloseConversation))
                                    (:1
                                      (CallFunction|DiceRollSeduction 4)
                                      (CallFunction|ClearDialogueProgress)
                                      (CallFunction|CloseConversation))
                                    (:2
                                      (CallFunction|ClearDialogueProgress)
                                      (CallFunction|CloseConversation))))))
                            (:2
                              (CallFunction|RemoveDialogueProgress 1))))))
                    (:1
                      (CallFunction|DiceRollSeduction 2)
                      ;[1 1 1] Bloque de conversacion (2)
                      (bind (_state_6 _optionsindex_6) (CallFunction|AddDialogue (Variables|Default|GetNPC%20Name) "Great, I have a book" (Utilities|Array|MakeArray "Con_2" "" "Back")))
                      (switch Utilities|FlowControl|Switch|SwitchonEnum_DialogueState _state_6
                        (:NewEnumerator0
                          (switch int _optionsindex_6
                            (:0
                              (CallFunction|DiceRollAgresion 3)
                              ;[1 1 1] Bloque de conversacion (3)
                              (bind (_state_7 _optionsindex_7) (CallFunction|AddDialogue (Variables|Default|GetNPC%20Name) "What makes Sherlock special?" (Utilities|Array|MakeArray "Aggressive: Holmes's deductive brilliance." "Seduction: Solving impossible cases." "Bye!")))
                              (switch Utilities|FlowControl|Switch|SwitchonEnum_DialogueState _state_7
                                (:NewEnumerator0
                                  (switch int _optionsindex_7
                                    (:0
                                      (CallFunction|DiceRollAgresion 4)
                                      (CallFunction|ClearDialogueProgress)
                                      (CallFunction|CloseConversation))
                                    (:1
                                      (CallFunction|DiceRollSeduction 4)
                                      (CallFunction|ClearDialogueProgress)
                                      (CallFunction|CloseConversation))
                                    (:2
                                      (CallFunction|ClearDialogueProgress)
                                      (CallFunction|CloseConversation))))))
                            (:1
                              (CallFunction|DiceRollSeduction 3)
                              ;[1 1 1] Bloque de conversacion (3)
                              (bind (_state_8 _optionsindex_8) (CallFunction|AddDialogue (Variables|Default|GetNPC%20Name) "What makes Sherlock special?" (Utilities|Array|MakeArray "Aggressive: Holmes's deductive brilliance." "Seduction: Solving impossible cases." "Bye!")))
                              (switch Utilities|FlowControl|Switch|SwitchonEnum_DialogueState _state_8
                                (:NewEnumerator0
                                  (switch int _optionsindex_8
                                    (:0
                                      (CallFunction|DiceRollAgresion 4)
                                      (CallFunction|ClearDialogueProgress)
                                      (CallFunction|CloseConversation))
                                    (:1
                                      (CallFunction|DiceRollSeduction 4)
                                      (CallFunction|ClearDialogueProgress)
                                      (CallFunction|CloseConversation))
                                    (:2
                                      (CallFunction|ClearDialogueProgress)
                                      (CallFunction|CloseConversation))))))
                            (:2
                              (CallFunction|RemoveDialogueProgress 1))))))
                    (:2
                      (CallFunction|RemoveDialogueProgress 1))))))
            (:1
              (CallFunction|DiceRollSeduction 1)
              ;[1 1 1] Bloque de conversacion (1)
              (bind (_state_9 _optionsindex_9) (CallFunction|AddDialogue (Variables|Default|GetNPC%20Name) "Too bad, I have a book" (Utilities|Array|MakeArray "I dont wanted" "" "Back")))
              (switch Utilities|FlowControl|Switch|SwitchonEnum_DialogueState _state_9
                (:NewEnumerator0
                  (switch int _optionsindex_9
                    (:0
                      (CallFunction|DiceRollAgresion 2)
                      ;[1 1 1] Bloque de conversacion (2)
                      (bind (_state_10 _optionsindex_10) (CallFunction|AddDialogue (Variables|Default|GetNPC%20Name) "What makes Sherlock special?" (Utilities|Array|MakeArray "Aggressive: Holmes's deductive brilliance." "Seduction: Solving impossible cases." "Back")))
                      (switch Utilities|FlowControl|Switch|SwitchonEnum_DialogueState _state_10
                        (:NewEnumerator0
                          (switch int _optionsindex_10
                            (:0
                              (CallFunction|DiceRollAgresion 3)
                              ;[1 1 1] Bloque de conversacion (3)
                              (bind (_state_11 _optionsindex_11) (CallFunction|AddDialogue (Variables|Default|GetNPC%20Name) "What makes Sherlock special?" (Utilities|Array|MakeArray "Aggressive: Holmes's deductive brilliance." "Seduction: Solving impossible cases." "Bye!")))
                              (switch Utilities|FlowControl|Switch|SwitchonEnum_DialogueState _state_11
                                (:NewEnumerator0
                                  (switch int _optionsindex_11
                                    (:0
                                      (CallFunction|DiceRollAgresion 4)
                                      (CallFunction|ClearDialogueProgress)
                                      (CallFunction|CloseConversation))
                                    (:1
                                      (CallFunction|DiceRollSeduction 4)
                                      (CallFunction|ClearDialogueProgress)
                                      (CallFunction|CloseConversation))
                                    (:2
                                      (CallFunction|ClearDialogueProgress)
                                      (CallFunction|CloseConversation))))))
                            (:1
                              (CallFunction|DiceRollSeduction 3)
                              ;[1 1 1] Bloque de conversacion (3)
                              (bind (_state_12 _optionsindex_12) (CallFunction|AddDialogue (Variables|Default|GetNPC%20Name) "What makes Sherlock special?" (Utilities|Array|MakeArray "Aggressive: Holmes's deductive brilliance." "Seduction: Solving impossible cases." "Bye!")))
                              (switch Utilities|FlowControl|Switch|SwitchonEnum_DialogueState _state_12
                                (:NewEnumerator0
                                  (switch int _optionsindex_12
                                    (:0
                                      (CallFunction|DiceRollAgresion 4)
                                      (CallFunction|ClearDialogueProgress)
                                      (CallFunction|CloseConversation))
                                    (:1
                                      (CallFunction|DiceRollSeduction 4)
                                      (CallFunction|ClearDialogueProgress)
                                      (CallFunction|CloseConversation))
                                    (:2
                                      (CallFunction|ClearDialogueProgress)
                                      (CallFunction|CloseConversation))))))
                            (:2
                              (CallFunction|RemoveDialogueProgress 1))))))
                    (:1
                      (CallFunction|DiceRollSeduction 2)
                      ;[1 1 1] Bloque de conversacion (2)
                      (bind (_state_13 _optionsindex_13) (CallFunction|AddDialogue (Variables|Default|GetNPC%20Name) "Great, I have a book" (Utilities|Array|MakeArray "Con_2" "" "Back")))
                      (switch Utilities|FlowControl|Switch|SwitchonEnum_DialogueState _state_13
                        (:NewEnumerator0
                          (switch int _optionsindex_13
                            (:0
                              (CallFunction|DiceRollAgresion 3)
                              ;[1 1 1] Bloque de conversacion (3)
                              (bind (_state_14 _optionsindex_14) (CallFunction|AddDialogue (Variables|Default|GetNPC%20Name) "What makes Sherlock special?" (Utilities|Array|MakeArray "Aggressive: Holmes's deductive brilliance." "Seduction: Solving impossible cases." "Bye!")))
                              (switch Utilities|FlowControl|Switch|SwitchonEnum_DialogueState _state_14
                                (:NewEnumerator0
                                  (switch int _optionsindex_14
                                    (:0
                                      (CallFunction|DiceRollAgresion 4)
                                      (CallFunction|ClearDialogueProgress)
                                      (CallFunction|CloseConversation))
                                    (:1
                                      (CallFunction|DiceRollSeduction 4)
                                      (CallFunction|ClearDialogueProgress)
                                      (CallFunction|CloseConversation))
                                    (:2
                                      (CallFunction|ClearDialogueProgress)
                                      (CallFunction|CloseConversation))))))
                            (:1
                              (CallFunction|DiceRollSeduction 3)
                              ;[1 1 1] Bloque de conversacion (3)
                              (bind (_state_15 _optionsindex_15) (CallFunction|AddDialogue (Variables|Default|GetNPC%20Name) "What makes Sherlock special?" (Utilities|Array|MakeArray "Aggressive: Holmes's deductive brilliance." "Seduction: Solving impossible cases." "Bye!")))
                              (switch Utilities|FlowControl|Switch|SwitchonEnum_DialogueState _state_15
                                (:NewEnumerator0
                                  (switch int _optionsindex_15
                                    (:0
                                      (CallFunction|DiceRollAgresion 4)
                                      (CallFunction|ClearDialogueProgress)
                                      (CallFunction|CloseConversation))
                                    (:1
                                      (CallFunction|DiceRollSeduction 4)
                                      (CallFunction|ClearDialogueProgress)
                                      (CallFunction|CloseConversation))
                                    (:2
                                      (CallFunction|ClearDialogueProgress)
                                      (CallFunction|CloseConversation))))))
                            (:2
                              (CallFunction|RemoveDialogueProgress 1))))))
                    (:2
                      (CallFunction|RemoveDialogueProgress 1))))))
            (:2
              (CallFunction|ClearDialogueProgress)
              (CallFunction|CloseConversation))))))))