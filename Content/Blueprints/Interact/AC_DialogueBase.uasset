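; Base dialogue component that runs branching NPC conversations in WB_NPCs, with an empty Dialogue function for child scripts.
; Each choice is stored in DialogueProgress, then Dialogue replays from the start, skipping answered steps until it shows the next unanswered one.
; Seduction and aggression dice rolls shift NPC and player emotions by willpower comparison, granting XP on player wins.
; BeginPlay caches the first BP_NPC_V2 found, not necessarily the owner, and the player.
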(event EventBeginPlay
  (bind _outactors (Actor|GetAllActorsOfClass "/Game/Blueprints/NPCs/BP_NPC_V2.BP_NPC_V2_C"))
  (Variables|Default|SetNPCs (Utilities|Array|Get(acopy) _outactors))
  (bind _outactors_2 (Actor|GetAllActorsOfClass "/Game/ThirdPerson/Blueprints/BP_ThirdPersonCharacter.BP_ThirdPersonCharacter_C"))
  (Variables|Default|SetPlayer (Utilities|Array|Get(acopy) _outactors_2)))

(fn Dialogue)

(fn OpenConversation
  (bind _returnvalue (UserInterface|CreateWidget "/Game/Blueprints/UI/WB_NPCs.WB_NPCs_C" 0 self))
  (bind _output_get (Variables|Default|SetDialogueWidget _returnvalue))
  (UserInterface|Viewport|AddtoViewport _output_get 0)
  (Dialogue|ProgressDialogue))

(fn ProgressDialogue
  (Variables|Default|SetDialogueIndex -1)
  (Dialogue|Dialogue))

(fn CloseConversation
  (Widget|RemovefromParent (Variables|Default|GetDialogueWidget))
  (Class|BPIInteractable|ConversationClosed(Message) (Components|GetOwner)))

(fn AddDialogue
  (params (NPC%20Name :type Text) (Dialogue :type Text) (OptionsText :type Array%20of%20Texts))
  (bind _dialogueprogress (Variables|Default|GetDialogueProgress))
  (bind _dialogueindex (Variables|Default|GetDialogueIndex))
  (bind (_value _returnvalue) (Utilities|Map|Find _dialogueprogress _dialogueindex))
  (Math|Integer|IncrementInt _dialogueindex
    (:%20%20
      (if _returnvalue
        (return "NewEnumerator0" _value)
        (else
          (Default|UpdateDialogueText (Variables|Default|GetDialogueWidget) _dialogueindex NPC%20Name Dialogue OptionsText)
          (return "NewEnumerator1" 0))))))

(fn UpdateSelectedOption
  (params (ProgressIndex :type Integer%20%28by%20ref%29) (OptionsIndex :type Integer%20%28by%20ref%29))
  (Utilities|Map|Add (Variables|Default|GetDialogueProgress) ProgressIndex OptionsIndex)
  (Dialogue|ProgressDialogue))

(fn ClearDialogueProgress
  (Utilities|Map|Clear (Variables|Default|GetDialogueProgress)))

(fn RemoveDialogueProgress
  (params (ProgressSteps :type Integer))
  (for _index (range 0 ProgressSteps)
    (Utilities|Map|Remove (Variables|Default|GetDialogueProgress) (- (Variables|Default|GetDialogueIndex) _index))))

(fn SetDialogueTreeIndex
  (params (DialogueTreeIndex :type Integer))
  (Variables|Default|SetDialogueTreeIndex DialogueTreeIndex)
  (Dialogue|ClearDialogueProgress))

(fn DiceRollSeduction
  (params (OptionsPosition :type Integer))
  (bind _player (Variables|Default|GetPlayer))
  (bind _npcs (Variables|Default|GetNPCs))
  (bind _player_2 (Variables|Default|GetPlayer))
  (bind _npcs_2 (Variables|Default|GetNPCs))
  (bind _npcs_3 (Variables|Default|GetNPCs))
  (bind _player_3 (Variables|Default|GetPlayer))
  (bind _npcs_4 (Variables|Default|GetNPCs))
  (bind _npcs_5 (Variables|Default|GetNPCs))
  (bind _npcs_6 (Variables|Default|GetNPCs))
  (bind _npcs_7 (Variables|Default|GetNPCs))
  (bind _npcs_8 (Variables|Default|GetNPCs))
  (bind _player_4 (Variables|Default|GetPlayer))
  (bind _player_5 (Variables|Default|GetPlayer))
  (bind _npcs_9 (Variables|Default|GetNPCs))
  (bind _player_6 (Variables|Default|GetPlayer))
  (bind _player_7 (Variables|Default|GetPlayer))
  (bind _player_8 (Variables|Default|GetPlayer))
  (bind _player_9 (Variables|Default|GetPlayer))
  (bind _player_10 (Variables|Default|GetPlayer))
  (bind _npcs_10 (Variables|Default|GetNPCs))
  (bind _player_11 (Variables|Default|GetPlayer))
  (bind _player_12 (Variables|Default|GetPlayer))
  (bind _npcs_11 (Variables|Default|GetNPCs))
  (bind _npcs_12 (Variables|Default|GetNPCs))
  ;[1 1 1] Posicion de la conversacion
  (if (== OptionsPosition (Utilities|Map|Length (Variables|Default|GetDialogueProgress)))
    ;[1 1 1] NPC < Player
    (if (< (Variables|/Game/Blueprints/NPCs/BP_NPC_V2.BP_NPC_V2_C|GetnpcWillpower (Variables|Default|GetNPCs)) (Variables|/Game/ThirdPerson/Blueprints/BP_ThirdPersonCharacter.BP_ThirdPersonCharacter_C|GetplayerWillpower (Variables|Default|GetPlayer)))
      ;[1 1 1] Tirada de dado
      (if (> (Math|Random|RandomIntegerinRange 1 6) 3)
        (Utilities|FlowControl|Sequence
          (:then_0
            ;[1 1 1] NPC win
            (Variables|/Game/Blueprints/NPCs/BP_NPC_V2.BP_NPC_V2_C|SetnpcSadness _npcs_3 (+ (Variables|/Game/Blueprints/NPCs/BP_NPC_V2.BP_NPC_V2_C|GetnpcSadness _npcs_10) 15))
            (Variables|/Game/Blueprints/NPCs/BP_NPC_V2.BP_NPC_V2_C|SetnpcHappiness _npcs_3 (+ (Variables|/Game/Blueprints/NPCs/BP_NPC_V2.BP_NPC_V2_C|GetnpcHappiness _npcs_10) 15)))
          (:then_1
            (Variables|/Game/ThirdPerson/Blueprints/BP_ThirdPersonCharacter.BP_ThirdPersonCharacter_C|SetplayerSadness _player_6 (- (Variables|/Game/ThirdPerson/Blueprints/BP_ThirdPersonCharacter.BP_ThirdPersonCharacter_C|GetplayerSadness _player_11) 10))
            (Variables|/Game/ThirdPerson/Blueprints/BP_ThirdPersonCharacter.BP_ThirdPersonCharacter_C|SetplayerHappiness _player_6 (- (Variables|/Game/ThirdPerson/Blueprints/BP_ThirdPersonCharacter.BP_ThirdPersonCharacter_C|GetplayerHappiness _player_11) 10))))
        (else
          (Utilities|FlowControl|Sequence
            (:then_0
              ;[0 1 0.03412] Player win
              (Variables|/Game/Blueprints/NPCs/BP_NPC_V2.BP_NPC_V2_C|SetnpcSadness _npcs_4 (- (Variables|/Game/Blueprints/NPCs/BP_NPC_V2.BP_NPC_V2_C|GetnpcSadness _npcs_8) 15))
              (Variables|/Game/Blueprints/NPCs/BP_NPC_V2.BP_NPC_V2_C|SetnpcHappiness _npcs_4 (- (Variables|/Game/Blueprints/NPCs/BP_NPC_V2.BP_NPC_V2_C|GetnpcHappiness _npcs_8) 15)))
            (:then_1
              (Variables|/Game/ThirdPerson/Blueprints/BP_ThirdPersonCharacter.BP_ThirdPersonCharacter_C|SetplayerSadness _player_7 (+ (Variables|/Game/ThirdPerson/Blueprints/BP_ThirdPersonCharacter.BP_ThirdPersonCharacter_C|GetplayerSadness _player_4) 10))
              (Variables|/Game/ThirdPerson/Blueprints/BP_ThirdPersonCharacter.BP_ThirdPersonCharacter_C|SetplayerHappiness _player_7 (+ (Variables|/Game/ThirdPerson/Blueprints/BP_ThirdPersonCharacter.BP_ThirdPersonCharacter_C|GetplayerHappiness _player_4) 10))
              (Variables|/Game/ThirdPerson/Blueprints/BP_ThirdPersonCharacter.BP_ThirdPersonCharacter_C|SetXP _player_7 (+ (Variables|/Game/ThirdPerson/Blueprints/BP_ThirdPersonCharacter.BP_ThirdPersonCharacter_C|GetXP _player_7) 0.2))))))
      (else
        ;[1 1 1] NPC = Player
        (if (== (Variables|/Game/Blueprints/NPCs/BP_NPC_V2.BP_NPC_V2_C|GetnpcWillpower (Variables|Default|GetNPCs)) (Variables|/Game/ThirdPerson/Blueprints/BP_ThirdPersonCharacter.BP_ThirdPersonCharacter_C|GetplayerWillpower (Variables|Default|GetPlayer)))
          ;[1 1 1] Tirada de dado
          (if (> (Math|Random|RandomIntegerinRange 1 6) 3)
            (Utilities|FlowControl|Sequence
              (:then_0
                ;[1 1 1] NPC win
                (Variables|/Game/Blueprints/NPCs/BP_NPC_V2.BP_NPC_V2_C|SetnpcSadness _npcs_5 (+ (Variables|/Game/Blueprints/NPCs/BP_NPC_V2.BP_NPC_V2_C|GetnpcSadness _npcs_12) 10))
                (Variables|/Game/Blueprints/NPCs/BP_NPC_V2.BP_NPC_V2_C|SetnpcHappiness _npcs_5 (+ (Variables|/Game/Blueprints/NPCs/BP_NPC_V2.BP_NPC_V2_C|GetnpcHappiness _npcs_12) 10)))
              (:then_1
                (Variables|/Game/ThirdPerson/Blueprints/BP_ThirdPersonCharacter.BP_ThirdPersonCharacter_C|SetplayerSadness _player_8 (- (Variables|/Game/ThirdPerson/Blueprints/BP_ThirdPersonCharacter.BP_ThirdPersonCharacter_C|GetplayerSadness _player) 7))
                (Variables|/Game/ThirdPerson/Blueprints/BP_ThirdPersonCharacter.BP_ThirdPersonCharacter_C|SetplayerHappiness _player_8 (- (Variables|/Game/ThirdPerson/Blueprints/BP_ThirdPersonCharacter.BP_ThirdPersonCharacter_C|GetplayerHappiness _player) 7))))
            (else
              (Utilities|FlowControl|Sequence
                (:then_0
                  ;[0 1 0.03412] Player win
                  (Variables|/Game/Blueprints/NPCs/BP_NPC_V2.BP_NPC_V2_C|SetnpcSadness _npcs_6 (- (Variables|/Game/Blueprints/NPCs/BP_NPC_V2.BP_NPC_V2_C|GetnpcSadness _npcs_9) 10))
                  (Variables|/Game/Blueprints/NPCs/BP_NPC_V2.BP_NPC_V2_C|SetnpcHappiness _npcs_6 (- (Variables|/Game/Blueprints/NPCs/BP_NPC_V2.BP_NPC_V2_C|GetnpcHappiness _npcs_9) 10)))
                (:then_1
                  (Variables|/Game/ThirdPerson/Blueprints/BP_ThirdPersonCharacter.BP_ThirdPersonCharacter_C|SetplayerSadness _player_9 (+ (Variables|/Game/ThirdPerson/Blueprints/BP_ThirdPersonCharacter.BP_ThirdPersonCharacter_C|GetplayerSadness _player_5) 7))
                  (Variables|/Game/ThirdPerson/Blueprints/BP_ThirdPersonCharacter.BP_ThirdPersonCharacter_C|SetplayerHappiness _player_9 (+ (Variables|/Game/ThirdPerson/Blueprints/BP_ThirdPersonCharacter.BP_ThirdPersonCharacter_C|GetplayerHappiness _player_5) 7))
                  (Variables|/Game/ThirdPerson/Blueprints/BP_ThirdPersonCharacter.BP_ThirdPersonCharacter_C|SetXP _player_9 (+ (Variables|/Game/ThirdPerson/Blueprints/BP_ThirdPersonCharacter.BP_ThirdPersonCharacter_C|GetXP _player_9) 0.3))))))
          (else
            ;[1 1 1] NPC > Player
            (if (> (Variables|/Game/Blueprints/NPCs/BP_NPC_V2.BP_NPC_V2_C|GetnpcWillpower (Variables|Default|GetNPCs)) (Variables|/Game/ThirdPerson/Blueprints/BP_ThirdPersonCharacter.BP_ThirdPersonCharacter_C|GetplayerWillpower (Variables|Default|GetPlayer)))
              ;[1 1 1] Tirada de dado
              (if (> (Math|Random|RandomIntegerinRange 1 6) 3)
                (Utilities|FlowControl|Sequence
                  (:then_0
                    ;[1 1 1] NPC win
                    (Variables|/Game/Blueprints/NPCs/BP_NPC_V2.BP_NPC_V2_C|SetnpcSadness _npcs_7 (+ (Variables|/Game/Blueprints/NPCs/BP_NPC_V2.BP_NPC_V2_C|GetnpcSadness _npcs) 5))
                    (Variables|/Game/Blueprints/NPCs/BP_NPC_V2.BP_NPC_V2_C|SetnpcHappiness _npcs_7 (+ (Variables|/Game/Blueprints/NPCs/BP_NPC_V2.BP_NPC_V2_C|GetnpcHappiness _npcs) 5)))
                  (:then_1
                    (Variables|/Game/ThirdPerson/Blueprints/BP_ThirdPersonCharacter.BP_ThirdPersonCharacter_C|SetplayerSadness _player_10 (- (Variables|/Game/ThirdPerson/Blueprints/BP_ThirdPersonCharacter.BP_ThirdPersonCharacter_C|GetplayerSadness _player_12) 3))
                    (Variables|/Game/ThirdPerson/Blueprints/BP_ThirdPersonCharacter.BP_ThirdPersonCharacter_C|SetplayerHappiness _player_10 (- (Variables|/Game/ThirdPerson/Blueprints/BP_ThirdPersonCharacter.BP_ThirdPersonCharacter_C|GetplayerHappiness _player_12) 3))))
                (else
                  (Utilities|FlowControl|Sequence
                    (:then_0
                      ;[0 1 0.03412] Player win
                      (Variables|/Game/Blueprints/NPCs/BP_NPC_V2.BP_NPC_V2_C|SetnpcSadness _npcs_2 (- (Variables|/Game/Blueprints/NPCs/BP_NPC_V2.BP_NPC_V2_C|GetnpcSadness _npcs_11) 5))
                      (Variables|/Game/Blueprints/NPCs/BP_NPC_V2.BP_NPC_V2_C|SetnpcHappiness _npcs_2 (- (Variables|/Game/Blueprints/NPCs/BP_NPC_V2.BP_NPC_V2_C|GetnpcHappiness _npcs_11) 5)))
                    (:then_1
                      (Variables|/Game/ThirdPerson/Blueprints/BP_ThirdPersonCharacter.BP_ThirdPersonCharacter_C|SetplayerSadness _player_3 (+ (Variables|/Game/ThirdPerson/Blueprints/BP_ThirdPersonCharacter.BP_ThirdPersonCharacter_C|GetplayerSadness _player_2) 3))
                      (Variables|/Game/ThirdPerson/Blueprints/BP_ThirdPersonCharacter.BP_ThirdPersonCharacter_C|SetplayerHappiness _player_3 (+ (Variables|/Game/ThirdPerson/Blueprints/BP_ThirdPersonCharacter.BP_ThirdPersonCharacter_C|GetplayerHappiness _player_2) 3))
                      (Variables|/Game/ThirdPerson/Blueprints/BP_ThirdPersonCharacter.BP_ThirdPersonCharacter_C|SetXP _player_3 (+ (Variables|/Game/ThirdPerson/Blueprints/BP_ThirdPersonCharacter.BP_ThirdPersonCharacter_C|GetXP _player_3) 0.4)))))))))))))

(fn DiceRollAgresion
  (params (OptionsPosition :type Integer))
  (bind _player (Variables|Default|GetPlayer))
  (bind _npcs (Variables|Default|GetNPCs))
  (bind _player_2 (Variables|Default|GetPlayer))
  (bind _npcs_2 (Variables|Default|GetNPCs))
  (bind _npcs_3 (Variables|Default|GetNPCs))
  (bind _player_3 (Variables|Default|GetPlayer))
  (bind _npcs_4 (Variables|Default|GetNPCs))
  (bind _npcs_5 (Variables|Default|GetNPCs))
  (bind _npcs_6 (Variables|Default|GetNPCs))
  (bind _npcs_7 (Variables|Default|GetNPCs))
  (bind _npcs_8 (Variables|Default|GetNPCs))
  (bind _player_4 (Variables|Default|GetPlayer))
  (bind _player_5 (Variables|Default|GetPlayer))
  (bind _npcs_9 (Variables|Default|GetNPCs))
  (bind _player_6 (Variables|Default|GetPlayer))
  (bind _player_7 (Variables|Default|GetPlayer))
  (bind _player_8 (Variables|Default|GetPlayer))
  (bind _player_9 (Variables|Default|GetPlayer))
  (bind _player_10 (Variables|Default|GetPlayer))
  (bind _npcs_10 (Variables|Default|GetNPCs))
  (bind _player_11 (Variables|Default|GetPlayer))
  (bind _player_12 (Variables|Default|GetPlayer))
  (bind _npcs_11 (Variables|Default|GetNPCs))
  (bind _npcs_12 (Variables|Default|GetNPCs))
  ;[1 1 1] Posicion de la conversacion
  (if (== OptionsPosition (Utilities|Map|Length (Variables|Default|GetDialogueProgress)))
    ;[1 1 1] NPC < Player
    (if (< (Variables|/Game/Blueprints/NPCs/BP_NPC_V2.BP_NPC_V2_C|GetnpcWillpower (Variables|Default|GetNPCs)) (Variables|/Game/ThirdPerson/Blueprints/BP_ThirdPersonCharacter.BP_ThirdPersonCharacter_C|GetplayerWillpower (Variables|Default|GetPlayer)))
      ;[1 1 1] Tirada de dado
      (if (>= (Math|Random|RandomIntegerinRange -1 6) 3)
        (Utilities|FlowControl|Sequence
          (:then_0
            ;[1 1 1] NPC win
            (Variables|/Game/Blueprints/NPCs/BP_NPC_V2.BP_NPC_V2_C|SetnpcAffection _npcs_3 (+ (Variables|/Game/Blueprints/NPCs/BP_NPC_V2.BP_NPC_V2_C|GetnpcAffection _npcs_10) 15))
            (Variables|/Game/Blueprints/NPCs/BP_NPC_V2.BP_NPC_V2_C|SetnpcAggression _npcs_3 (+ (Variables|/Game/Blueprints/NPCs/BP_NPC_V2.BP_NPC_V2_C|GetnpcAggression _npcs_10) 15)))
          (:then_1
            (Variables|/Game/ThirdPerson/Blueprints/BP_ThirdPersonCharacter.BP_ThirdPersonCharacter_C|SetplayerAffection _player_6 (- (Variables|/Game/ThirdPerson/Blueprints/BP_ThirdPersonCharacter.BP_ThirdPersonCharacter_C|GetplayerAffection _player_11) 7))
            (Variables|/Game/ThirdPerson/Blueprints/BP_ThirdPersonCharacter.BP_ThirdPersonCharacter_C|SetplayerAggression _player_6 (- (Variables|/Game/ThirdPerson/Blueprints/BP_ThirdPersonCharacter.BP_ThirdPersonCharacter_C|GetplayerAggression _player_11) 7))))
        (else
          (Utilities|FlowControl|Sequence
            (:then_0
              ;[0 1 0.03412] Player win
              (Variables|/Game/Blueprints/NPCs/BP_NPC_V2.BP_NPC_V2_C|SetnpcAffection _npcs_4 (- (Variables|/Game/Blueprints/NPCs/BP_NPC_V2.BP_NPC_V2_C|GetnpcAffection _npcs_8) 15))
              (Variables|/Game/Blueprints/NPCs/BP_NPC_V2.BP_NPC_V2_C|SetnpcAggression _npcs_4 (- (Variables|/Game/Blueprints/NPCs/BP_NPC_V2.BP_NPC_V2_C|GetnpcAggression _npcs_8) 15)))
            (:then_1
              (Variables|/Game/ThirdPerson/Blueprints/BP_ThirdPersonCharacter.BP_ThirdPersonCharacter_C|SetplayerAffection _player_7 (+ (Variables|/Game/ThirdPerson/Blueprints/BP_ThirdPersonCharacter.BP_ThirdPersonCharacter_C|GetplayerAffection _player_4) 10))
              (Variables|/Game/ThirdPerson/Blueprints/BP_ThirdPersonCharacter.BP_ThirdPersonCharacter_C|SetplayerAggression _player_7 (+ (Variables|/Game/ThirdPerson/Blueprints/BP_ThirdPersonCharacter.BP_ThirdPersonCharacter_C|GetplayerAggression _player_4) 10))
              (Variables|/Game/ThirdPerson/Blueprints/BP_ThirdPersonCharacter.BP_ThirdPersonCharacter_C|SetXP _player_7 (+ (Variables|/Game/ThirdPerson/Blueprints/BP_ThirdPersonCharacter.BP_ThirdPersonCharacter_C|GetXP _player_7) 0.2))))))
      (else
        ;[1 1 1] NPC = Player
        (if (== (Variables|/Game/Blueprints/NPCs/BP_NPC_V2.BP_NPC_V2_C|GetnpcWillpower (Variables|Default|GetNPCs)) (Variables|/Game/ThirdPerson/Blueprints/BP_ThirdPersonCharacter.BP_ThirdPersonCharacter_C|GetplayerWillpower (Variables|Default|GetPlayer)))
          ;[1 1 1] Tirada de dado
          (if (>= (Math|Random|RandomIntegerinRange 0 6) 3)
            (Utilities|FlowControl|Sequence
              (:then_0
                ;[1 1 1] NPC win
                (Variables|/Game/Blueprints/NPCs/BP_NPC_V2.BP_NPC_V2_C|SetnpcAffection _npcs_5 (+ (Variables|/Game/Blueprints/NPCs/BP_NPC_V2.BP_NPC_V2_C|GetnpcAffection _npcs_12) 10))
                (Variables|/Game/Blueprints/NPCs/BP_NPC_V2.BP_NPC_V2_C|SetnpcAggression _npcs_5 (+ (Variables|/Game/Blueprints/NPCs/BP_NPC_V2.BP_NPC_V2_C|GetnpcAggression _npcs_12) 10)))
              (:then_1
                (Variables|/Game/ThirdPerson/Blueprints/BP_ThirdPersonCharacter.BP_ThirdPersonCharacter_C|SetplayerAffection _player_8 (- (Variables|/Game/ThirdPerson/Blueprints/BP_ThirdPersonCharacter.BP_ThirdPersonCharacter_C|GetplayerAffection _player) 5))
                (Variables|/Game/ThirdPerson/Blueprints/BP_ThirdPersonCharacter.BP_ThirdPersonCharacter_C|SetplayerAggression _player_8 (- (Variables|/Game/ThirdPerson/Blueprints/BP_ThirdPersonCharacter.BP_ThirdPersonCharacter_C|GetplayerAggression _player) 5))))
            (else
              (Utilities|FlowControl|Sequence
                (:then_0
                  ;[0 1 0.03412] Player win
                  (Variables|/Game/Blueprints/NPCs/BP_NPC_V2.BP_NPC_V2_C|SetnpcAffection _npcs_6 (- (Variables|/Game/Blueprints/NPCs/BP_NPC_V2.BP_NPC_V2_C|GetnpcAffection _npcs_9) 10))
                  (Variables|/Game/Blueprints/NPCs/BP_NPC_V2.BP_NPC_V2_C|SetnpcAggression _npcs_6 (- (Variables|/Game/Blueprints/NPCs/BP_NPC_V2.BP_NPC_V2_C|GetnpcAggression _npcs_9) 10)))
                (:then_1
                  (Variables|/Game/ThirdPerson/Blueprints/BP_ThirdPersonCharacter.BP_ThirdPersonCharacter_C|SetplayerAffection _player_9 (+ (Variables|/Game/ThirdPerson/Blueprints/BP_ThirdPersonCharacter.BP_ThirdPersonCharacter_C|GetplayerAffection _player_5) 7))
                  (Variables|/Game/ThirdPerson/Blueprints/BP_ThirdPersonCharacter.BP_ThirdPersonCharacter_C|SetplayerAggression _player_9 (+ (Variables|/Game/ThirdPerson/Blueprints/BP_ThirdPersonCharacter.BP_ThirdPersonCharacter_C|GetplayerAggression _player_5) 7))
                  (Variables|/Game/ThirdPerson/Blueprints/BP_ThirdPersonCharacter.BP_ThirdPersonCharacter_C|SetXP _player_9 (+ (Variables|/Game/ThirdPerson/Blueprints/BP_ThirdPersonCharacter.BP_ThirdPersonCharacter_C|GetXP _player_9) 0.3))))))
          (else
            ;[1 1 1] NPC > Player
            (if (> (Variables|/Game/Blueprints/NPCs/BP_NPC_V2.BP_NPC_V2_C|GetnpcWillpower (Variables|Default|GetNPCs)) (Variables|/Game/ThirdPerson/Blueprints/BP_ThirdPersonCharacter.BP_ThirdPersonCharacter_C|GetplayerWillpower (Variables|Default|GetPlayer)))
              ;[1 1 1] Tirada de dado
              (if (>= (Math|Random|RandomIntegerinRange 1 6) 3)
                (Utilities|FlowControl|Sequence
                  (:then_0
                    ;[1 1 1] NPC win
                    (Variables|/Game/Blueprints/NPCs/BP_NPC_V2.BP_NPC_V2_C|SetnpcAffection _npcs_7 (+ (Variables|/Game/Blueprints/NPCs/BP_NPC_V2.BP_NPC_V2_C|GetnpcAffection _npcs) 5))
                    (Variables|/Game/Blueprints/NPCs/BP_NPC_V2.BP_NPC_V2_C|SetnpcAggression _npcs_7 (+ (Variables|/Game/Blueprints/NPCs/BP_NPC_V2.BP_NPC_V2_C|GetnpcAggression _npcs) 5)))
                  (:then_1
                    (Variables|/Game/ThirdPerson/Blueprints/BP_ThirdPersonCharacter.BP_ThirdPersonCharacter_C|SetplayerAffection _player_10 (- (Variables|/Game/ThirdPerson/Blueprints/BP_ThirdPersonCharacter.BP_ThirdPersonCharacter_C|GetplayerAffection _player_12) 3))
                    (Variables|/Game/ThirdPerson/Blueprints/BP_ThirdPersonCharacter.BP_ThirdPersonCharacter_C|SetplayerAggression _player_10 (- (Variables|/Game/ThirdPerson/Blueprints/BP_ThirdPersonCharacter.BP_ThirdPersonCharacter_C|GetplayerAggression _player_12) 3))))
                (else
                  (Utilities|FlowControl|Sequence
                    (:then_0
                      ;[0 1 0.03412] Player win
                      (Variables|/Game/Blueprints/NPCs/BP_NPC_V2.BP_NPC_V2_C|SetnpcAffection _npcs_2 (- (Variables|/Game/Blueprints/NPCs/BP_NPC_V2.BP_NPC_V2_C|GetnpcAffection _npcs_11) 5))
                      (Variables|/Game/Blueprints/NPCs/BP_NPC_V2.BP_NPC_V2_C|SetnpcAggression _npcs_2 (- (Variables|/Game/Blueprints/NPCs/BP_NPC_V2.BP_NPC_V2_C|GetnpcAggression _npcs_11) 5)))
                    (:then_1
                      (Variables|/Game/ThirdPerson/Blueprints/BP_ThirdPersonCharacter.BP_ThirdPersonCharacter_C|SetplayerAffection _player_3 (+ (Variables|/Game/ThirdPerson/Blueprints/BP_ThirdPersonCharacter.BP_ThirdPersonCharacter_C|GetplayerAffection _player_2) 5))
                      (Variables|/Game/ThirdPerson/Blueprints/BP_ThirdPersonCharacter.BP_ThirdPersonCharacter_C|SetplayerAggression _player_3 (+ (Variables|/Game/ThirdPerson/Blueprints/BP_ThirdPersonCharacter.BP_ThirdPersonCharacter_C|GetplayerAggression _player_2) 5))
                      (Variables|/Game/ThirdPerson/Blueprints/BP_ThirdPersonCharacter.BP_ThirdPersonCharacter_C|SetXP _player_3 (+ (Variables|/Game/ThirdPerson/Blueprints/BP_ThirdPersonCharacter.BP_ThirdPersonCharacter_C|GetXP _player_3) 0.4)))))))))))))